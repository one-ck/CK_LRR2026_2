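; BP_CameraFOV visualizes a cine camera's field of view as lines between a near and a far plane, built entirely in the Construction Script.
; The camera's focal length, scaled up, places the nodal point, with the far plane twice as far out.
; Four line components aim from near corners to opposite far corners, suggesting rays crossing at the nodal point.
; All four stretch by the same A-to-D diagonal distance, scaled to extend the lines.
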(event EventBeginPlay)

(event Collision|EventActorBeginOverlap
  (params (OtherActor :type Actor%20Object%20Reference)))

(event EventTick
  (params (DeltaSeconds :type Float%20%28single-precision%29)))

(fn ConstructionScript
  (bind _linelooka (Variables|Default|GetLineLookA))
  (bind _nearposa (Variables|Default|GetNearPosA))
  (bind _farposd (Variables|Default|GetFarPosD))
  (bind _linelookb (Variables|Default|GetLineLookB))
  (bind _linelookc (Variables|Default|GetLineLookC))
  (bind _linelookd (Variables|Default|GetLineLookD))
  (bind _returnvalue (Transformation|GetWorldLocation _nearposa))
  (bind _returnvalue_2 (Transformation|GetWorldLocation _farposd))
  (bind _returnvalue_3 (Math|Vector|Distance(Vector) _returnvalue _returnvalue_2))
  (bind _returnvalue_4 (* _returnvalue_3 0.02))
  (bind _returnvalue_5 (Math|Vector|MakeVector _returnvalue_4 0.1 0.1))
  (bind _ascine_camera_component (Utilities|Casting|CastToCineCameraComponent (Variables|CameraActor|GetCameraComponent)))
  (Transformation|SetRelativeLocation (Variables|Default|GetNodalPoint) (Math|Vector|MakeVector (* (Variables|/Script/CinematicCamera.CineCameraComponent|GetCurrentFocalLength _ascine_camera_component) 4.0) 0.0 0.0) false false)
  (Transformation|SetRelativeLocation (Variables|Default|GetFarPlane) (Math|Vector|MakeVector (* (* (Variables|/Script/CinematicCamera.CineCameraComponent|GetCurrentFocalLength _ascine_camera_component) 4.0) 2.0) 0.0 0.0) false false)
  (Transformation|SetWorldRotation _linelooka (Math|Rotator|FindLookatRotation _returnvalue _returnvalue_2) false false)
  (Transformation|SetRelativeScale3D _linelooka _returnvalue_5)
  (Transformation|SetWorldRotation _linelookb (Math|Rotator|FindLookatRotation (Transformation|GetWorldLocation (Variables|Default|GetNearPosB)) (Transformation|GetWorldLocation (Variables|Default|GetFarPosC))) false false)
  (Transformation|SetRelativeScale3D _linelookb _returnvalue_5)
  (Transformation|SetWorldRotation _linelookc (Math|Rotator|FindLookatRotation (Transformation|GetWorldLocation (Variables|Default|GetNearPosC)) (Transformation|GetWorldLocation (Variables|Default|GetFarPosB))) false false)
  (Transformation|SetRelativeScale3D _linelookc _returnvalue_5)
  (Transformation|SetWorldRotation _linelookd (Math|Rotator|FindLookatRotation (Transformation|GetWorldLocation (Variables|Default|GetNearPosD)) (Transformation|GetWorldLocation (Variables|Default|GetFarPosA))) false false)
  (Transformation|SetRelativeScale3D _linelookd _returnvalue_5))